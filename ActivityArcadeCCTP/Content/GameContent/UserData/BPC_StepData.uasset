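; BPC_StepData is an actor component that stores the player's step count and ticket count.
; Two events, StepsUpdated and UpdateTickets, add the given amount to the running total.
; Each then casts the owner to BP_TopDownCharacter and its controller to BP_TopDownController to push the new total to the GameUI step or ticket display.
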(event Custom|UpdateTickets
  (params (UpdateAmount :type Integer))
  ;[1 1 1 1 58] UPDATE TICKET VARIABLE + UI
  (Variables|Default|SetStoredTickets (+ UpdateAmount (Variables|Default|GetStoredTickets)))
  (bind _asbp_top_down_character (Utilities|Casting|CastToBP_TopDownCharacter (Components|GetOwner)))
  (bind _asbp_top_down_controller (Utilities|Casting|CastToBP_TopDownController (Pawn|GetController _asbp_top_down_character)))
  (Default|UpdateTicketUI (Variables|/Game/TopDown/Blueprints/BP_TopDownController.BP_TopDownController_C|GetGameUI _asbp_top_down_controller) (Variables|Default|GetStoredTickets)))

(event Custom|StepsUpdated
  (params (UpdateAmount :type Integer))
  ;[1 1 1 1 50] UPDATE STEPS VARIABLES + UI
  (Variables|Default|SetUserSteps (+ UpdateAmount (Variables|Default|GetUserSteps)))
  (bind _asbp_top_down_character (Utilities|Casting|CastToBP_TopDownCharacter (Components|GetOwner)))
  (bind _asbp_top_down_controller (Utilities|Casting|CastToBP_TopDownController (Pawn|GetController _asbp_top_down_character)))
  (Default|UpdateStepUI (Variables|/Game/TopDown/Blueprints/BP_TopDownController.BP_TopDownController_C|GetGameUI _asbp_top_down_controller) (Variables|Default|GetUserSteps)))